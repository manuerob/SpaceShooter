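; An obstacle actor that explodes on contact and triggers game over when the player's spaceship hits it.
; Any overlap with its Box spawns a Niagara burst at its location and destroys the actor before the spaceship pawn cast runs.
; For a spaceship, a FlipFlop first opens the GameOver_BP widget, pauses and shows the cursor; its alternate branch reverses this.
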(event OnComponentBeginOverlap(Box)
  (params (OverlappedComponent :type Primitive%20Component%20Object%20Reference) (OtherActor :type Actor%20Object%20Reference) (OtherComp :type Primitive%20Component%20Object%20Reference) (OtherBodyIndex :type Integer) (bFromSweep :type Boolean) (SweepResult :type Hit%20Result%20Structure%20%28by%20ref%29))
  (bind _returnvalue (Game|GetPlayerController 0))
  (Niagara|SpawnSystematLocation "/Game/Materials/OmniBurstNiagara_System1.OmniBurstNiagara_System1" (Transformation|GetActorLocation))
  (Actor|DestroyActor)
  (Utilities|Casting|CastToSSM_Spaceship_Pawn OtherActor)
  (if true
    ;[1 1 1] Game Over Menu
    (Utilities|FlowControl|FlipFlop
      (:A
        (bind _returnvalue_2 (UserInterface|CreateWidget "/Game/HUD/GameOver_BP.GameOver_BP_C"))
        (UserInterface|Viewport|AddtoViewport _returnvalue_2 0)
        (Game|SetGamePaused true)
        (Variables|/Script/Engine.PlayerController|SetbShowMouseCursor _returnvalue true))
      (:B
        (Widget|RemovefromParent _returnvalue_2)
        (Game|SetGamePaused false)
        (Variables|/Script/Engine.PlayerController|SetbShowMouseCursor _returnvalue false)))))

(event EventBeginPlay)

(event Collision|EventActorBeginOverlap
  (params (OtherActor :type Actor%20Object%20Reference)))

(event EventTick
  (params (DeltaSeconds :type Float%20%28single-precision%29)))

(fn ConstructionScript)